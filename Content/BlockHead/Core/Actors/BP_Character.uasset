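; Player character for BlockHead that is pushed forward automatically and steered side to side until the level ends.
; Movement applies forces to a near-frictionless CharacterMovement component, with steering only while on a blocking floor.
; Hitting an obstacle (after a short delay) or falling below a custom kill height triggers PlayerDied, while overlapping the end point completes the level.
; Both outcomes set LevelEnded and notify BP_GameMode.
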(event OnComponentHit(CapsuleComponent)
  (params (HitComponent :type Primitive%20Component%20Object%20Reference) (OtherActor :type Actor%20Object%20Reference) (OtherComp :type Primitive%20Component%20Object%20Reference) (NormalImpulse :type Vector :default "0, 0, 0") (Hit :type Hit%20Result%20Structure%20%28by%20ref%29))
  ;[0.09561 1 0.1374] Player Hits an Obstacle
  (Utilities|Casting|CastToBP_Obstacle OtherActor)
  (Utilities|FlowControl|Delay 0.2)
  (CallFunction|PlayerDied))

(event OnComponentBeginOverlap(CapsuleComponent)
  (params (OverlappedComponent :type Primitive%20Component%20Object%20Reference) (OtherActor :type Actor%20Object%20Reference) (OtherComp :type Primitive%20Component%20Object%20Reference) (OtherBodyIndex :type Integer) (bFromSweep :type Boolean) (SweepResult :type Hit%20Result%20Structure%20%28by%20ref%29))
  (Utilities|Casting|CastToBP_EndPoint OtherActor)
  (Variables|Default|SetbLevelEnded true)
  (Default|LevelComplete (Variables|Default|GetAs%20BP%20Game%20Mode)))

(event EventBeginPlay
  ;[0.09561 1 0.1374] On Begin Play
  (Utilities|FlowControl|Sequence
    (:then_0
      ;;[0.09561 1 0.1374] Reduce Character Movement Friction
      (Variables|/Script/Engine.CharacterMovementComponent|SetGroundFriction (Variables|Character|GetCharacterMovement) 0.001)
      (Variables|/Script/Engine.CharacterMovementComponent|SetBrakingDecelerationWalking (Variables|Character|GetCharacterMovement) 2048.0))
    (:then_1
      ;;[0.09561 1 0.1374] Save Reference to Game Mode
      (bind _asbp_game_mode (Utilities|Casting|CastToBP_GameMode (Game|GetGameMode)))
      (Variables|Default|SetAs%20BP%20Game%20Mode _asbp_game_mode))))

(event EventTick
  (params (DeltaSeconds :type Float%20%28single-precision%29))
  ;[0.09561 1 0.1374] Character Movement
  ;;[0.09561 1 0.1374] Forward Motion on Tick
  (if (not (Variables|Default|GetbLevelEnded))
    (Physics|AddForce (Variables|Character|GetCharacterMovement) (Math|Vector|MakeVector (Variables|Default|GetForwardForce) 0.0 0.0))
    ;;[0.09561 1 0.1374] Custom Kill Z
    (if (< (.z (Transformation|GetActorLocation)) -75.0)
      (CallFunction|PlayerDied))))

(event Input|AxisEvents|InputAxisMoveLeftRight
  (params (AxisValue :type Float%20%28single-precision%29))
  ;[0.09561 1 0.1374] Character Movement
  ;;[0.09561 1 0.1374] Side to Side Motion
  (if (not (Variables|Default|GetbLevelEnded))
    (if (.bblockinghit (Variables|/Script/Engine.CharacterMovementComponent|GetCurrentFloor (Variables|Character|GetCharacterMovement)))
      (Physics|AddForce (Variables|Character|GetCharacterMovement) (Math|Vector|MakeVector 0.0 (* (Input|AxisValues|GetMoveLeftRight) (Variables|Default|GetSideForce)) 0.0)))))

(fn ConstructionScript)

(fn PlayerDied
  ;[0.09561 1 0.1374] Player Died Function
  (if (not (Variables|Default|GetbLevelEnded))
    (Variables|Default|SetbLevelEnded true)
    (Default|LoadGameCompleteScreen (Variables|Default|GetAs%20BP%20Game%20Mode) false)
    (return)))