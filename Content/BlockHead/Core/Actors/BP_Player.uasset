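; BP_Player is the BlockHead player cube, pushed constantly forward by physics while the player steers it sideways.
; Tick applies forward force and checks a kill-Z height, while the MoveLeftRight axis applies side force, both as acceleration changes.
; Hitting a BP_Obstacle or falling calls PlayerDied, and overlapping BP_EndPoint completes the level.
; A LevelEnded flag stops movement and repeat deaths, with outcomes reported to BP_GameMode.
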(event OnComponentHit(PlayerCube)
  (params (HitComponent :type Primitive%20Component%20Object%20Reference) (OtherActor :type Actor%20Object%20Reference) (OtherComp :type Primitive%20Component%20Object%20Reference) (NormalImpulse :type Vector :default "0, 0, 0") (Hit :type Hit%20Result%20Structure%20%28by%20ref%29))
  ;[0.09561 1 0.1374] Hits and Overlaps
  ;;[0.09561 1 0.1374] Player Hits an Obstacle
  (Utilities|Casting|CastToBP_Obstacle OtherActor)
  (CallFunction|PlayerDied))

(event OnComponentBeginOverlap(PlayerCube)
  (params (OverlappedComponent :type Primitive%20Component%20Object%20Reference) (OtherActor :type Actor%20Object%20Reference) (OtherComp :type Primitive%20Component%20Object%20Reference) (OtherBodyIndex :type Integer) (bFromSweep :type Boolean) (SweepResult :type Hit%20Result%20Structure%20%28by%20ref%29))
  ;[0.09561 1 0.1374] Hits and Overlaps
  ;;[0.09561 1 0.1374] Player Completed Level Successfully
  (Utilities|Casting|CastToBP_EndPoint OtherActor)
  (Variables|Default|SetbLevelEnded true)
  (Default|LevelComplete (Variables|Default|GetAs%20BP%20Game%20Mode)))

(event EventTick
  (params (DeltaSeconds :type Float%20%28single-precision%29))
  ;[0.09561 1 0.1374] Motion Code
  ;;[0.09561 1 0.1374] Constant Character Forward Movement (ON TICK)
  (if (not (Variables|Default|GetbLevelEnded))
    (Physics|AddForce (Variables|Default|GetPlayerCube) (Math|Vector|MakeVector (Variables|Default|GetForwardForce) 0.0 0.0) "None" true)
    ;;[0.09561 1 0.1374] Kill Z
    (if (< (.z (Transformation|GetActorLocation)) -35.0)
      (CallFunction|PlayerDied))))

(event EventBeginPlay
  ;[0.09561 1 0.1374] Get Reference to Game Mode on Begin Play
  (bind _asbp_game_mode (Utilities|Casting|CastToBP_GameMode (Game|GetGameMode)))
  (Variables|Default|SetAs%20BP%20Game%20Mode _asbp_game_mode))

(event Input|AxisEvents|InputAxisMoveLeftRight
  (params (AxisValue :type Float%20%28single-precision%29))
  ;[0.09561 1 0.1374] Motion Code
  ;;[0.09561 1 0.1374] User-Controlled Sideways Character Motion
  (if (not (Variables|Default|GetbLevelEnded))
    (Physics|AddForce (Variables|Default|GetPlayerCube) (Math|Vector|MakeVector 0.0 (* AxisValue (Variables|Default|GetSideForce)) 0.0) "None" true)))

(fn ConstructionScript)

(fn PlayerDied
  ;[0.9474 1 0.236] Player Died Function
  (if (not (Variables|Default|GetbLevelEnded))
    (Variables|Default|SetbLevelEnded true)
    (Default|EndGame (Variables|Default|GetAs%20BP%20Game%20Mode))))