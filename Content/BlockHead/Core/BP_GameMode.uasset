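; BlockHead game mode that manages level flow and the win/lose end screens.
; On begin play it adds the HUD, caches BP_GameInstance and sets game-only input with a hidden cursor.
; LevelComplete shows a widget, then a timer calls LoadNextLevel, which opens the next level or shows the win screen after the final one.
; EndGame shows the loss screen; RestartGame resets the game instance's level counter and reopens that level.
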(event EventBeginPlay
  (bind _returnvalue (Game|GetPlayerController 0))
  (Utilities|FlowControl|Sequence
    (:then_0
      ;[0.09561 1 0.1374] Add HUD to Viewport
      (bind _returnvalue_2 (UserInterface|CreateWidget "/Game/BlockHead/Core/UI/WBP_HUD.WBP_HUD_C"))
      (bind _output_get (Variables|Default|SetHUD _returnvalue_2))
      (UserInterface|Viewport|AddtoViewport _output_get 0))
    (:then_1
      ;[0.09561 1 0.1374] Get Reference to the Global Game Instance
      (bind _asbp_game_instance (Utilities|Casting|CastToBP_GameInstance (Game|GetGameInstance)))
      (Variables|Default|SetBP%20Game%20Instance _asbp_game_instance))
    (:then_2
      ;[0.09561 1 0.1374] Hide Mouse Pointer and Set Input to Game Only
      (Variables|/Script/Engine.PlayerController|SetbShowMouseCursor _returnvalue false)
      (Input|SetInputModeGameOnly _returnvalue))))

(fn ConstructionScript)

(fn EndGame
  ;[0.09561 1 0.1374] Game Over. Display Game Complete Screen
  (CallFunction|LoadGameCompleteScreen false))

(fn LevelComplete
  ;[0.09561 1 0.1374] When BP_Player Indicates Level is Complete Show Complete Widget and then Load Next Level
  (bind _returnvalue (UserInterface|CreateWidget "/Game/BlockHead/Core/UI/WBP_LevelComplete.WBP_LevelComplete_C"))
  (UserInterface|Viewport|AddtoViewport _returnvalue 0)
  (Utilities|Time|SetTimerbyFunctionName 0 "LoadNextLevel" 2.0))

(fn LoadNextLevel
  ;[1 1 1] Comment
  (bind _bfinallevel (Default|IsPlayeronFinalLevel (Variables|Default|GetBP%20Game%20Instance)))
  (if _bfinallevel
    (CallFunction|LoadGameCompleteScreen true)
    (else
      (Default|IncreaseLevel (Variables|Default|GetBP%20Game%20Instance))
      (bind _levelname (Default|GetLevelName (Variables|Default|GetBP%20Game%20Instance)))
      (Game|OpenLevel(byName) _levelname))))

(fn RestartGame
  ;[0.09561 1 0.1374] Restart Game By Way of Game Instance
  (Default|ResetLevelCounter (Variables|Default|GetBP%20Game%20Instance))
  (bind _levelname (Default|GetLevelName (Variables|Default|GetBP%20Game%20Instance)))
  (Game|OpenLevel(byName) _levelname))

(fn LoadGameCompleteScreen
  (params (bPlayerWon :type Boolean))
  ;[0.09561 1 0.1374] Show Game Complete Screen with Win or Loss Message
  (if bPlayerWon
    (LocalVariables|SetCustomMessage "You Win!")
    (else
      (LocalVariables|SetCustomMessage "You Lose!")))
  (bind _returnvalue (UserInterface|CreateWidget "/Game/BlockHead/Core/UI/WBP_GameComplete.WBP_GameComplete_C"))
  (Variables|Default|SetWBP%20Game%20Complete _returnvalue)
  (Rendering|Components|TextRender|SetText (Variables|/Game/BlockHead/Core/UI/WBP_GameComplete.WBP_GameComplete_C|GetLostOrComplete (Variables|Default|GetWBP%20Game%20Complete)) (LocalVariables|GetCustomMessage))
  (UserInterface|Viewport|AddtoViewport (Variables|Default|GetWBP%20Game%20Complete) 0))